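; DCGameState is a Game State Blueprint that exposes server settings and decides whether networked events are still relevant by age and distance.
; Helpers compare elapsed server world time and vector distance against MaxLagTime and MaxCullDistance from ServerSettings.
; CheckNetRelevancy picks none, time, distance or both by enum, while IsNetRelevant tests both and always fails on dedicated servers.
; SendError prints error strings on screen, and the event graph is unused.
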(event EventBeginPlay)

(event EventTick
  (params (DeltaSeconds :type Float%20%28single-precision%29)))

(fn ConstructionScript)

(fn GetServerSettings
  (return (Variables|Default|GetServerSettings)))

(fn IsNetRelevantTime
  (params (InitTime :type Float%20%28single-precision%29))
  (return (<= (- (GameState|GetServerWorldTimeSeconds) InitTime) (Utilities|Struct|BreakF_ServerSettings (Variables|Default|GetServerSettings)))))

(fn IsNetRelevantDistance
  (params (VectorA :type Vector) (VectorB :type Vector))
  (return (<= (Math|Vector|VectorLength (- VectorA VectorB)) (Utilities|Struct|BreakF_ServerSettings (Variables|Default|GetServerSettings)))))

(fn IsNetRelevant
  (params (InitTime :type Float%20%28single-precision%29) (InitLocation :type Vector) (ReceiveLocation :type Vector))
  (if (Networking|IsDedicatedServer)
    (return false)
    (elif (<= (- (GameState|GetServerWorldTimeSeconds) InitTime) (Utilities|Struct|BreakF_ServerSettings (Variables|Default|GetServerSettings)))
      (if (<= (Math|Vector|VectorLength (- InitLocation ReceiveLocation)) (Utilities|Struct|BreakF_ServerSettings (Variables|Default|GetServerSettings)))
        (return true)
        (else
          (return false)))
      (else
        (return false)))))

(fn CheckNetRelevancy
  (params (NetRelevancy :type E_NetRelevancy%20Enum :default "NewEnumerator0") (Time :type Float%20%28single-precision%29) (DistA :type Vector) (DistB :type Vector))
  (bind _return_value (CallFunction|IsNetRelevantTime Time))
  (bind _return_value_2 (CallFunction|IsNetRelevantDistance DistA DistB))
  (switch Utilities|FlowControl|Switch|SwitchonE_NetRelevancy NetRelevancy
    (:NewEnumerator0
      (LocalVariables|SetReturnBool true))
    (:NewEnumerator1
      (LocalVariables|SetReturnBool _return_value))
    (:NewEnumerator2
      (LocalVariables|SetReturnBool _return_value_2))
    (:NewEnumerator3
      (LocalVariables|SetReturnBool (and _return_value _return_value_2))))
  (return (LocalVariables|GetReturnBool)))

(fn SendError
  (params (ErrorString :type String))
  (Development|PrintString (Utilities|String|Append "Error: " ErrorString) true true "(R=0.592126,G=0.000000,B=1.000000,A=1.000000)" 1e+01))