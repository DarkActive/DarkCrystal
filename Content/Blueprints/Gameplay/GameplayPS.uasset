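; GameplayPS is the gameplay player state, handling the switch to a newly selected weapon.
; The Equipment component's select event calls a server update that runs only with authority.
; It validates the weapon, feeds montages matching the character's gender to MontageManager, sets the right-hand mesh's anim class and toggles the weapon through GameplayPC.
; Invalid selections reset selection state and report an error via game state; IsAlive always returns true.
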(event OnWeaponSelect(Equipment)
  (params (Weapon :type F%20Weapon%20Structure))
  (CallFunction|ServerUpdateSelectedWeapon)
  (Development|PrintString "Cleint got OnWeaponSelect"))

(event Custom|Server_UpdateSelectedWeapon
  (Weapons|UpdatetoSelectedWeapon))

(fn ConstructionScript)

(fn IsAlive
  (return true))

(fn UpdatetoSelectedWeapon
  (bind _playercontroller (Helpers|GetOwnedController))
  (bind _equipment (Variables|Default|GetEquipment))
  (bind _character (Default|GetOwnedCharacter _playercontroller))
  (bind _weapon (Default|GetActiveWeapon _equipment))
  (bind _weapon_2 (Default|GetWeaponInfo _weapon))
  (bind _charactertype (Variables|/Game/Characters/BP_BaseCharacter.BP_BaseCharacter_C|GetCharacterType _character))
  (bind (_type _animationinstance _femalemontages _malemontages) (Utilities|Struct|BreakF_Weapon _weapon_2))
  (bind _returnvalue (Utilities|Select :Index _charactertype :NewEnumerator0 _femalemontages :NewEnumerator1 _malemontages))
  (Networking|SwitchHasAuthority
    (:Authority
      (if (Utilities|Enum|NotEqual(Enum) _type "NewEnumerator0")
        (Utilities|IsValid _returnvalue
          (:Is%20Valid
            (Default|UpdateMontages (Variables|Default|GetMontageManager) _returnvalue)
            (Components|SkeletalMesh|SetAnimInstanceClass (Variables|/Game/Characters/BP_BaseCharacter.BP_BaseCharacter_C|GetRightHandMesh _character) _animationinstance)
            (Variables|Default|SetIsSelectingWeapon false)
            (Variables|Default|SetOnSelectWeaponSlot "NewEnumerator4")
            (Default|ToggleWeapon _playercontroller))
          (:Is%20Not%20Valid
            (Variables|Default|SetIsSelectingWeapon false :!label _label)
            (Variables|Default|SetOnSelectWeaponSlot "NewEnumerator4")
            (Default|SendError (Utilities|GetGameState) "Selected weapon is invalid.")))
        (else
          (goto _label))))))

(fn GetOwnedController
  (return (.AsGameplay%20PC (Utilities|Casting|CastToGameplayPC (Components|GetOwner)))))