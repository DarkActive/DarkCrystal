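; BPC_MontageManager is a component that supplies animation montages for actions from a swappable Montages DataTable.
; Lookups convert the action enum to a row name, then return the montage at a clamped index with a success flag.
; Helpers return an action's last or random montage index, and UpdateMontages replaces the table.
; BeginPlay prints a warning naming the owner when the table is invalid.
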(event EventBeginPlay
  ;[1 1 1] Make sure DataTable is valid
  (Utilities|IsValid (Variables|Default|GetMontages)
    (:Is%20Not%20Valid
      (Development|PrintString (Utilities|String|Append "Montages DataTable on " (Utilities|GetDisplayName (Components|GetOwner)) " is Not Valid !")))))

(fn GetMontageforAction
  (params (Enumerator :type E_MontageAction%20Enum :default "NewEnumerator0") (Index :type Integer))
  (bind _montages (Variables|Default|GetMontages))
  ;[1 1 1] Returns montage at give index if it exists in table
  (Utilities|IsValid _montages
    (:Is%20Valid
      (bind _returnvalue (Utilities|GetDataTableRow _montages (Utilities|String|StringToName (Utilities|String|EnumtoString Enumerator)))
        (:then
          (Utilities|IsValid (Utilities|Array|Get(acopy) (.Montages (Utilities|Struct|BreakF_MontageAction _returnvalue)) (Math|Integer|Clamp(Integer) Index 0 (Utilities|Array|LastIndex (.Montages (Utilities|Struct|BreakF_MontageAction _returnvalue)))))
            (:Is%20Valid
              (return (Utilities|Array|Get(acopy) (.Montages (Utilities|Struct|BreakF_MontageAction _returnvalue)) (Math|Integer|Clamp(Integer) Index 0 (Utilities|Array|LastIndex (.Montages (Utilities|Struct|BreakF_MontageAction _returnvalue))))) true))
            (:Is%20Not%20Valid
              _)))
        (:RowNotFound
          _)))
    (:Is%20Not%20Valid
      _))
  (return 0 false))

(fn GetMontageActionLastIndex
  (params (Action :type E_MontageAction%20Enum :default "NewEnumerator0"))
  (bind _montages (Variables|Default|GetMontages))
  (Utilities|IsValid _montages
    (:Is%20Valid
      (bind _returnvalue (Utilities|GetDataTableRow _montages (Utilities|String|StringToName (Utilities|String|EnumtoString Action)))
        (:then
          (return (Utilities|Array|LastIndex (.Montages (Utilities|Struct|BreakF_MontageAction _returnvalue)))))
        (:RowNotFound
          _)))
    (:Is%20Not%20Valid
      _))
  (return 0))

(fn GetRandomMontageIndex
  (params (MontageAction :type E_MontageAction%20Enum :default "NewEnumerator0"))
  (return (Math|Random|RandomIntegerinRange 0 (CallFunction|GetMontageActionLastIndex MontageAction))))

(fn UpdateMontages
  (params (Montages :type Data%20Table%20Object%20Reference))
  (Variables|Default|SetMontages Montages))