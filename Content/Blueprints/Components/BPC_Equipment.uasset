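; BPC_Equipment is an equipment component that holds four weapon slots and an arrow slot, and tracks the active weapon.
; SelectWeapon switches to a filled slot and broadcasts OnWeaponSelect with its weapon info, otherwise printing a message.
; Getters resolve the active weapon and supply attack and arrow stats, with default struct fallbacks.
; UpdateWeapon and RemoveWeapon are unfinished stubs, and the arrow validity check always returns true.
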(event EventBeginPlay)

(event EventTick
  (params (DeltaSeconds :type Float%20%28single-precision%29)))

(fn UpdateWeapon
  (params (Weapon :type BP%20Base%20Weapon%20Object%20Reference) (Slot :type E_WeaponSlots%20Enum :default "NewEnumerator4"))
  (LocalVariables|SetLocalWeapon Weapon)
  (LocalVariables|SetLocalSlot Slot)
  (Utilities|IsValid (LocalVariables|GetLocalWeapon)
    (:Is%20Not%20Valid
      (Update|RemoveWeapon))))

(fn RemoveWeapon)

(fn SelectWeapon
  (params (WeaponSlot :type E_WeaponSlots%20Enum :default "NewEnumerator4"))
  ;[1 1 1] Check if new selected slot has a valid weapon, if conditions are true then change active slot and call OnWeaponSelect Event
  (bind _output_get (LocalVariables|SetLocalWeapon (Getters|GetWeaponbySlot WeaponSlot)))
  (Utilities|IsValid _output_get
    (:Is%20Valid
      (Variables|Default|SetActiveWeaponSlot WeaponSlot)
      (Default|CallOnWeaponSelect (Default|GetWeaponInfo (LocalVariables|GetLocalWeapon))))
    (:Is%20Not%20Valid
      (Development|PrintString "No Weapon Equipped in that Slot." true true "(R=0.000000,G=0.660000,B=1.000000,A=1.000000)" 5.0))))

(fn GetWeaponbySlot
  (params (Slot :type E_WeaponSlots%20Enum :default "NewEnumerator4"))
  (switch Utilities|FlowControl|Switch|SwitchonE_WeaponSlots Slot
    (:NewEnumerator0
      (LocalVariables|SetLocalWeapon (Variables|Default|GetWeaponSlot1)))
    (:NewEnumerator1
      (LocalVariables|SetLocalWeapon (Variables|Default|GetWeaponSlot2)))
    (:NewEnumerator2
      (LocalVariables|SetLocalWeapon (Variables|Default|GetWeaponSlot3)))
    (:NewEnumerator3
      (LocalVariables|SetLocalWeapon (Variables|Default|GetWeaponSlot4))))
  (return (LocalVariables|GetLocalWeapon)))

(fn GetActiveWeapon
  (return (Getters|GetWeaponbySlot (Variables|Default|GetActiveWeaponSlot))))

(fn GetActiveSlot
  (return (Variables|Default|GetActiveWeaponSlot)))

(fn GetAttackStats
  (bind _weapon (Getters|GetActiveWeapon))
  (if (Utilities|IsValid _weapon)
    (return (Default|GetWeaponInfo _weapon))
    (else
      (return (Utilities|Struct|MakeF_Weapon "NewEnumerator0" 0.0)))))

(fn GetArrowStats
  (if (Validation|AreArrowsValid-TD)
    (return (Default|GetArrowInfo (Variables|Default|GetArrowsSlot)))
    (else
      (return (Utilities|Struct|MakeF_Arrow 1e+01 "ArrowSocket" "QuiverSocket")))))

(fn AreArrowsValid-TD
  (return true))