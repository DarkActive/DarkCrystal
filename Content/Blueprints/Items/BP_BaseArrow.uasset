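; BP_BaseArrow is the base Blueprint for arrow items, supplying each arrow's data from a data table.
; GetArrowInfo looks up the row named by ItemID in DT_Arrows and returns it, or an empty result if no row matches.
; The event graph holds only disabled default events, and the construction script just calls its parent.
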(event EventBeginPlay
  (|CallParentFunction) ; This node is disabled and will not be called.\nDrag off pins to build functionality.
)

(event Collision|EventActorBeginOverlap
  (params (OtherActor :type Actor%20Object%20Reference))
  (|CallParentFunction OtherActor) ; This node is disabled and will not be called.\nDrag off pins to build functionality.
)

(event EventTick
  (params (DeltaSeconds :type Float%20%28single-precision%29))
  (|CallParentFunction DeltaSeconds) ; This node is disabled and will not be called.\nDrag off pins to build functionality.
)

(fn ConstructionScript
  (|CallParentFunction))

(fn GetArrowInfo
  (bind _returnvalue (Utilities|GetDataTableRow "/Game/Blueprints/DataTables/DT_Arrows.DT_Arrows" (Variables|Default|GetItemID))
    (:then
      (return _returnvalue))
    (:RowNotFound
      (return ""))))