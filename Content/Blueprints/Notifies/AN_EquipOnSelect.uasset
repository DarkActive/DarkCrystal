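; Anim notify that equips the weapon a character is selecting at a point in its animation.
; On firing, it casts the mesh owner to the 0_Base class and checks that a weapon selection is in progress.
; It then tells that character's Equipment to select the weapon in the pending slot.
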(fn GetNotifyName
  (return "EquipOnSelect"))

(fn ReceivedNotify
  (params (MeshComp :type Skeletal%20Mesh%20Component%20Object%20Reference) (Animation :type Anim%20Sequence%20Base%20Object%20Reference))
  (bind _returnvalue (Components|GetOwner MeshComp))
  (Utilities|IsValid _returnvalue
    (:Is%20Valid
      (bind _as0_base (Utilities|Casting|CastTo0_Base _returnvalue))
      (if (Variables|/Game/Blueprints/Characters/0_Base.0_Base_C|GetIsSelectingWeapon _as0_base)
        (Default|SelectWeapon (Variables|/Game/Blueprints/Characters/0_Base.0_Base_C|GetEquipment _as0_base) (Variables|/Game/Blueprints/Characters/0_Base.0_Base_C|GetOnSelectWeaponSlot _as0_base))
        (return true)))))